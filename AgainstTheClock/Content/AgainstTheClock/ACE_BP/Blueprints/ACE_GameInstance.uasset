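; Game instance for Against the Clock that records clears, medals and ability unlocks for three levels.
; LevelCompletedEvent switches on level number and grades the time, higher values earning better medals, with each medal also granting those below.
; Level 1 gold unlocks wall jump and Level 2 gold unlocks double jump.
; Level 2's gold check uses OR instead of AND, so any non-negative minute count earns gold.
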(event Custom|LevelCompletedEvent
  (params (LevelNumber :type Integer) (Minutes :type Integer) (Seconds :type Integer))
  (switch int LevelNumber
    (:1
      ;[1 1 1] Level 1 cleared
      ;;[1 1 1] Gold
      (if (and (>= Minutes 0) (>= Seconds 27))
        (Variables|Default|SetLevel1Gold true)
        (Variables|Default|SetWallJumpUnlocked true)
        (Variables|Default|SetLevel1Silver true :!label _label)
        (else
          ;;[1 1 1] Silver
          (if (and (>= Minutes 0) (>= Seconds 15))
            (goto _label)
            (else
              _))))
      (Variables|Default|SetLevel1Bronze true)
      (Variables|Default|SetLevel1Cleared true))
    (:2
      ;[1 1 1] Level 2 cleared
      ;;[1 1 1] Gold
      (if (or (>= Minutes 0) (>= Seconds 55))
        (Variables|Default|SetLevel2Gold true)
        (Variables|Default|SetDoubleJumpUnlocked true)
        (Variables|Default|SetLevel2Silver true :!label _label_2)
        (else
          ;;[1 1 1] Silver
          (if (and (>= Minutes 0) (>= Seconds 35))
            (goto _label_2)
            (else
              _))))
      (Variables|Default|SetLevel2Bronze true)
      (Variables|Default|SetLevel2Cleared true))
    (:3
      ;[1 1 1] Level 3 cleared
      ;;[1 1 1] Gold
      (if (>= Minutes 1)
        (Variables|Default|SetLevel3Gold true)
        (Variables|Default|SetLevel3Silver true :!label _label_3)
        (else
          ;;[1 1 1] Silver
          (if (and (>= Minutes 0) (>= Seconds 50))
            (goto _label_3)
            (else
              _))))
      (Variables|Default|SetLevel3Bronze true)
      (Variables|Default|SetLevel3Cleared true))))