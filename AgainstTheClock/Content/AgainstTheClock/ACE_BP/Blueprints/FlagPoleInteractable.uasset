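; Level-end flagpole interactable that completes the current level when the player presses the Pickup(Interact) input inside its Box trigger.
; Box overlap toggles the actor's input for any actor, while a Gate opens and closes only for ThirdPersonCharacter.
; A gated press flags LevelCompleted on ACE_GameInstance, passes the character's CurrentLevelNumber to LevelCompletedEvent, then opens the Main_Menu_Levels map.
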(event OnComponentBeginOverlap(Box)
  (params (OverlappedComponent :type Primitive%20Component%20Object%20Reference) (OtherActor :type Actor%20Object%20Reference) (OtherComp :type Primitive%20Component%20Object%20Reference) (OtherBodyIndex :type Integer) (bFromSweep :type Boolean) (SweepResult :type Hit%20Result%20Structure%20%28by%20ref%29))
  (Input|EnableInput (Game|GetPlayerController 0))
  (Utilities|Casting|CastToThirdPersonCharacter OtherActor)
  (Utilities|FlowControl|Gate true) ; enters at Open
)

(event OnComponentEndOverlap(Box)
  (params (OverlappedComponent :type Primitive%20Component%20Object%20Reference) (OtherActor :type Actor%20Object%20Reference) (OtherComp :type Primitive%20Component%20Object%20Reference) (OtherBodyIndex :type Integer))
  (Input|DisableInput (Game|GetPlayerController 0))
  (Utilities|Casting|CastToThirdPersonCharacter OtherActor)
  (Utilities|FlowControl|Gate true) ; enters at Close
)

(event EventTick
  (params (DeltaSeconds :type Float%20%28single-precision%29)))

(event Collision|EventActorBeginOverlap
  (params (OtherActor :type Actor%20Object%20Reference)))

(event Input|ActionEvents|InputActionPickup(Interact)
  (params (Key :type Key%20Structure :default "None"))
  (:Pressed
    (Utilities|FlowControl|Gate true
      (:Exit
        (Development|PrintString "Item PickedUp")
        (bind _asace_game_instance (Utilities|Casting|CastToACE_GameInstance (Game|GetGameInstance)))
        (Variables|/Game/AgainstTheClock/ACE_BP/Blueprints/ACE_GameInstance.ACE_GameInstance_C|SetLevelCompleted _asace_game_instance true)
        (bind _asthird_person_character (Utilities|Casting|CastToThirdPersonCharacter (Game|Player|GetPlayerPawn 0)))
        (bind _asace_game_instance_2 (Utilities|Casting|CastToACE_GameInstance (Game|GetGameInstance)))
        (Default|LevelCompletedEvent _asace_game_instance_2 (Variables|/Game/AgainstTheClock/ACE_BP/Blueprints/ThirdPersonCharacter.ThirdPersonCharacter_C|GetCurrentLevelNumber _asthird_person_character))
        (Game|OpenLevel(byName) "Main_Menu_Levels")))))

(fn ConstructionScript)